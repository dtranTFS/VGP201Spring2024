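; Health component for the FPS game that stores clamped health and exposes damage, heal, death-check and normalized-health functions.
; Damage and Heal ignore negative amounts and route through ClampSetHealth to stay between zero and MaxHealth.
; BeginPlay initializes full health, then applies hardcoded damage, while Tick uses a Delay to heal at a steady interval.
; An unconnected graph holds an unused COD-style regeneration with a wait before healing.
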(event EventBeginPlay
  (CallFunction|Init (Variables|Setup|GetMaxHealth))
  (CallFunction|Damage 5e+01))

(event EventTick
  (params (DeltaSeconds :type Float%20%28single-precision%29))
  (Utilities|FlowControl|Delay (Variables|Setup|GetHealthRegenRate))
  (CallFunction|Heal (Variables|Setup|GetHealthRegenAmount)))

(fn Init
  (params (MaxHealth :type Float%20%28double-precision%29))
  (Variables|Setup|SetHealth MaxHealth))

(fn GetHealth
  (return (Variables|Setup|GetHealth)))

(fn Damage
  (params (Amount :type Float%20%28double-precision%29))
  (if (not (< Amount 0.0))
    (Utilities|ClampSetHealth (- (Variables|Setup|GetHealth) Amount))))

(fn Heal
  (params (Amount :type Float%20%28double-precision%29))
  (if (not (< Amount 0.0))
    (Utilities|ClampSetHealth (+ (Variables|Setup|GetHealth) Amount))))

(fn IsDead
  (return (<= (Variables|Setup|GetHealth) 0.0)))

(fn GetNormalizedHealth
  (return (Math|Float|Clamp(Float) (/ (Variables|Setup|GetHealth) (Variables|Setup|GetMaxHealth)))))