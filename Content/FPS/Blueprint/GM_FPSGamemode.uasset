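; Game mode for the FPS game that sets up the HUD and tracks the score.
; BeginPlay prints a debug message, adds the reticle and game UI widgets to the viewport, then initializes the health bar to full and shows the current score.
; AddScore adds points to the score and pushes the new total to the stored game UI widget.
; A countdown demo remains in the graph but never runs.
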(event EventBeginPlay
  (Development|PrintString "Spawning FPSGameMode" true true "(R=1.000000,G=0.000000,B=0.026793,A=1.000000)" 5.0)
  (bind _returnvalue (UserInterface|CreateWidget "/Game/FPS/Blueprint/GUI/WBP_Reticle.WBP_Reticle_C"))
  (UserInterface|Viewport|AddtoViewport _returnvalue 0)
  (bind _returnvalue_2 (UserInterface|CreateWidget "/Game/FPS/Blueprint/GUI/WBP_GameUI.WBP_GameUI_C"))
  (bind _output_get (Variables|Default|SetGameUI _returnvalue_2))
  (UserInterface|Viewport|AddtoViewport _output_get 0)
  (Default|SetHealthBar (Variables|Default|GetGameUI) 1.0)
  (Default|SetScore (Variables|Default|GetGameUI) (Variables|Default|GetScore)))

(event EventTick
  (params (DeltaSeconds :type Float%20%28single-precision%29)))

(fn ConstructionScript)

(fn AddScore
  (params (Points :type Integer))
  (bind _output_get (Variables|Default|SetScore (+ (Variables|Default|GetScore) Points)))
  (Default|SetScore (Variables|Default|GetGameUI) _output_get))